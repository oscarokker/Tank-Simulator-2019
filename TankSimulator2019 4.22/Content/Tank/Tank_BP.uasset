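; Tank Blueprint that sets up the turret and barrel and provides an orbiting aim camera.
; On BeginPlay it registers both components through the turret and barrel reference setters and assigns their static meshes.
; Azimuth input yaws the gimbal and elevation input pitches the spring arm, each scaled by delta time for framerate-independent rotation.
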(event EventBeginPlay
  (Class|Tank|SetTurretReference (Variables|Default|GetTurret))
  (Components|StaticMesh|SetStaticMesh (Variables|Default|GetTurret) "/Game/Tank/tank_fbx_Turret.tank_fbx_Turret")
  (Class|Tank|SetBarrelReference (Variables|Default|GetTankBarrel1))
  (Components|StaticMesh|SetStaticMesh (Variables|Default|GetTankBarrel1) "/Game/Tank/tank_fbx_Barrel.tank_fbx_Barrel"))

(event Input|AxisEvents|InputAxisAimAzimuth
  (params (AxisValue :type Float%20%28single-precision%29))
  ;[1 1 1] Camera input binding
  (Transformation|AddLocalRotation (Variables|Default|GetAzimuth%20Gimbale) (Math|Rotator|MakeRotator 0.0 0.0 (* AxisValue (Utilities|Time|GetWorldDeltaSeconds) 1e+02)) false false))

(event Input|AxisEvents|InputAxisAimElevation
  (params (AxisValue :type Float%20%28single-precision%29))
  ;[1 1 1] Camera input binding
  (Transformation|AddLocalRotation (Variables|Default|GetSpring%20Arm) (Math|Rotator|MakeRotator 0.0 (* AxisValue (Utilities|Time|GetWorldDeltaSeconds) 1e+02) 0.0) false false))

(fn ConstructionScript)